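; Homing missile actor that chases the player in the flying game and damages the player's flying pawn or a friendly jet on hit.
; Each tick it rolls, moves forward by a fixed per-frame step and interpolates rotation toward a lead point ahead of the player pawn.
; Those hits call ReduceHealth, stop the smoke, remove mesh and light, then destroy the actor after a delay.
; An out-of-range self-destruct check is present but unconnected.
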(event OnComponentHit(SM_Missile)
  (params (HitComponent :type Primitive%20Component%20Object%20Reference) (OtherActor :type Actor%20Object%20Reference) (OtherComp :type Primitive%20Component%20Object%20Reference) (NormalImpulse :type Vector :default "0, 0, 0") (Hit :type Hit%20Result%20Structure%20%28by%20ref%29))
  (bind _missiledamage (Variables|Default|GetMissileDamage))
  ;[1 1 1] damage
  (bind _astp_flying_pawn_bp (Utilities|Casting|CastToTP_FlyingPawn_BP OtherActor)
    (:then
      (Default|ReduceHealth _astp_flying_pawn_bp _missiledamage))
    (:CastFailed
      (bind _asfriendly_jet_bp (Utilities|Casting|CastToFriendlyJet_BP OtherActor))
      (Default|ReduceHealth _asfriendly_jet_bp _missiledamage)))
  (Components|Activation|Deactivate (Variables|Default|GetP_MissileSmoke))
  (Components|DestroyComponent (Variables|Default|GetSM_Missile))
  (Components|DestroyComponent (Variables|Default|GetPointLight))
  (Utilities|FlowControl|Delay 3.0)
  (Actor|DestroyActor))

(event EventTick
  (params (DeltaSeconds :type Float%20%28single-precision%29))
  (bind _returnvalue (Game|Player|GetPlayerPawn 0))
  (bind _defaultsceneroot (Variables|Default|GetDefaultSceneRoot))
  ;[1 1 1] Movement
  (Transformation|AddRelativeRotation (Variables|Default|GetDefaultSceneRoot) (Math|Rotator|MakeRotator (Variables|Default|GetSpinRate) 0.0 0.0) false false)
  (Transformation|SetActorLocation (+ (Transformation|GetActorLocation) (* (Transformation|GetActorForwardVector) (Variables|Default|GetMissileSpeed))) false false)
  (Transformation|SetWorldRotation _defaultsceneroot (Math|Interpolation|RInterpTo (Transformation|GetWorldRotation _defaultsceneroot) (Math|Rotator|FindLookatRotation (Transformation|GetWorldLocation _defaultsceneroot) (+ (* (Transformation|GetActorForwardVector _returnvalue) (Variables|Default|GetLeadDistance)) (Transformation|GetActorLocation _returnvalue))) DeltaSeconds (Variables|Default|GetMissileAgility)) false false))

(fn ConstructionScript)