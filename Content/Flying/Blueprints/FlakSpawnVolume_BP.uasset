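; Volume actor that continuously fills a box region with flak bursts by spawning FlakFire_BP actors.
; Tick drives a Delay of DeltaSeconds times SpawnRate, so SpawnRate acts roughly as a frame interval between spawns.
; Each spawn gets a random offset within the Volume box's scaled extent, added to the actor's location without applying its rotation.
; Spawned flak has random rotation and a fixed enlarged scale.
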(event EventBeginPlay)

(event Collision|EventActorBeginOverlap
  (params (OtherActor :type Actor%20Object%20Reference)))

(event EventTick
  (params (DeltaSeconds :type Float%20%28single-precision%29))
  (bind _volume (Variables|Default|GetVolume))
  (bind _returnvalue (Components|Box|GetScaledBoxExtent _volume))
  (bind (_x _y _z) (Math|Vector|BreakVector _returnvalue))
  (Utilities|FlowControl|Delay (* DeltaSeconds (Variables|Default|GetSpawnRate)))
  (Game|SpawnActorfromClass "/Game/Flying/Blueprints/FlakFire_BP.FlakFire_BP_C" (Math|Transform|MakeTransform (+ (Math|Vector|MakeVector (Math|Random|RandomFloatinRange (* _x -1.0) _x) (Math|Random|RandomFloatinRange (* _y -1.0) _y) (Math|Random|RandomFloatinRange (* _z -1.0) _z)) (Transformation|GetActorLocation)) (Math|Random|RandomRotator true) "10.000000,10.000000,10.000000") "Undefined" 0 0))

(fn ConstructionScript)