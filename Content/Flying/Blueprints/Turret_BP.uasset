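; Turret Blueprint that tracks the player pawn and fires bullets at it when within range.
; Tick eases the head's yaw and roll toward a point a fixed lead distance along the player's forward vector, with pitch locked to zero, and updates an in-range flag.
; A self-calling ShootAtPlayer loop, started on BeginPlay, spawns bullets from the barrel's Spawn socket at a set scale, paced by a retriggerable delay.
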(event Custom|ShootAtPlayer
  (bind _turret_barrels (Variables|Default|GetTurret_Barrels))
  (bind _returnvalue (Transformation|GetSocketTransform _turret_barrels "Spawn" "RTS_World"))
  (bind (_location _rotation) (Math|Transform|BreakTransform _returnvalue))
  (if (Variables|Default|GetInRange)
    (Game|SpawnActorfromClass (Variables|Default|GetBulletClass) (Math|Transform|MakeTransform _location _rotation (Variables|Default|GetBulletScale)) "Undefined" 0 0)
    (Utilities|FlowControl|RetriggerableDelay (Variables|Default|GetFireInterval))
    (CallFunction|ShootatPlayer)
    (else
      (Utilities|FlowControl|RetriggerableDelay (Variables|Default|GetFireInterval))
      (CallFunction|ShootatPlayer))))

(event EventBeginPlay
  (CallFunction|ShootatPlayer))

(event EventTick
  (params (DeltaSeconds :type Float%20%28single-precision%29))
  (bind _returnvalue (Game|Player|GetPlayerPawn 0))
  (bind _turret_head (Variables|Default|GetTurret_Head))
  (bind _leaddistance (Variables|Default|GetLeadDistance))
  (bind _returnvalue_2 (Transformation|GetWorldLocation _turret_head))
  (bind _returnvalue_3 (Transformation|GetActorForwardVector _returnvalue))
  (bind _returnvalue_4 (Transformation|GetActorLocation _returnvalue))
  (bind _returnvalue_5 (* _returnvalue_3 _leaddistance))
  (bind _returnvalue_6 (+ _returnvalue_5 _returnvalue_4))
  (bind _returnvalue_7 (Math|Rotator|FindLookatRotation _returnvalue_2 _returnvalue_6))
  (bind (_roll _pitch _yaw) (Math|Rotator|BreakRotator _returnvalue_7))
  ;[1 1 1] Rotation
  (Transformation|SetWorldRotation (Variables|Default|GetTurret_Head) (Math|Interpolation|RInterpTo (Transformation|GetWorldRotation _turret_head) (Math|Rotator|MakeRotator _roll 0.0 (+ _yaw 2.7e+02)) DeltaSeconds (Variables|Default|GetRotationSpeed)) false false)
  (if (< (Transformation|GetDistanceTo (Game|Player|GetPlayerPawn 0)) (Variables|Default|GetRange))
    (Variables|Default|SetInRange true)
    (else
      (Variables|Default|SetInRange false))))

(fn ConstructionScript)

(fn CopyRotations)