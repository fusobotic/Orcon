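; Projectile that damages the player's flying pawn or a friendly jet on impact.
; Each tick it moves forward by BulletSpeed with a swept location update, not scaled by delta time.
; A sphere hit calls ReduceHealth on either target type and destroys the bullet; other hits leave it alive.
; A kill-range check against player distance exists but is disconnected, so it never runs.
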(event OnComponentHit(Sphere)
  (params (HitComponent :type Primitive%20Component%20Object%20Reference) (OtherActor :type Actor%20Object%20Reference) (OtherComp :type Primitive%20Component%20Object%20Reference) (NormalImpulse :type Vector :default "0, 0, 0") (Hit :type Hit%20Result%20Structure%20%28by%20ref%29))
  (bind _bulletdamage (Variables|Default|GetBulletDamage))
  ;[1 1 1] damage
  (bind _astp_flying_pawn_bp (Utilities|Casting|CastToTP_FlyingPawn_BP OtherActor)
    (:then
      (Default|ReduceHealth _astp_flying_pawn_bp _bulletdamage))
    (:CastFailed
      (bind _asfriendly_jet_bp (Utilities|Casting|CastToFriendlyJet_BP OtherActor))
      (Default|ReduceHealth _asfriendly_jet_bp _bulletdamage)))
  (Actor|DestroyActor))

(event EventTick
  (params (DeltaSeconds :type Float%20%28single-precision%29))
  ;[1 1 1] Movement
  (Transformation|SetActorLocation (+ (Transformation|GetActorLocation) (* (Transformation|GetActorForwardVector) (Variables|Default|GetBulletSpeed))) true false))

(fn ConstructionScript)