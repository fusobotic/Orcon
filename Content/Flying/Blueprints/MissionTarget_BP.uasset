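; MissionTarget_BP is the Tupolev boss target of the flying mission, where the player can eject to finish.
; Overlapping EjectCol with the flying pawn sets EjectNow and shows the eject prompt on FlightHUD; leaving clears both.
; While inside, pressing E, J and C latches three flags, and Tick opens EndScreen once all are set.
; Hitting the Tupolev mesh with the pawn destroys this actor and reloads Level1.
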(event OnComponentBeginOverlap(EjectCol)
  (params (OverlappedComponent :type Primitive%20Component%20Object%20Reference) (OtherActor :type Actor%20Object%20Reference) (OtherComp :type Primitive%20Component%20Object%20Reference) (OtherBodyIndex :type Integer) (bFromSweep :type Boolean) (SweepResult :type Hit%20Result%20Structure%20%28by%20ref%29))
  (Utilities|Casting|CastToTP_FlyingPawn_BP OtherActor)
  (Variables|Default|SetEjectNow true)
  (bind _asflight_hud (Utilities|Casting|CastToFlightHUD (HUD|GetHUD (Game|GetPlayerController 0))))
  (Default|AddEject _asflight_hud))

(event OnComponentEndOverlap(EjectCol)
  (params (OverlappedComponent :type Primitive%20Component%20Object%20Reference) (OtherActor :type Actor%20Object%20Reference) (OtherComp :type Primitive%20Component%20Object%20Reference) (OtherBodyIndex :type Integer))
  (Utilities|Casting|CastToTP_FlyingPawn_BP OtherActor)
  (Variables|Default|SetEjectNow false)
  (bind _asflight_hud (Utilities|Casting|CastToFlightHUD (HUD|GetHUD (Game|GetPlayerController 0))))
  (Default|DeleteEject _asflight_hud))

(event OnComponentHit(SM_BossTupolev)
  (params (HitComponent :type Primitive%20Component%20Object%20Reference) (OtherActor :type Actor%20Object%20Reference) (OtherComp :type Primitive%20Component%20Object%20Reference) (NormalImpulse :type Vector :default "0, 0, 0") (Hit :type Hit%20Result%20Structure%20%28by%20ref%29))
  (Utilities|Casting|CastToTP_FlyingPawn_BP OtherActor)
  (Actor|DestroyActor)
  (Game|OpenLevel(byName) "Level1"))

(event EventTick
  (params (DeltaSeconds :type Float%20%28single-precision%29))
  (if (Math|Boolean|ANDBoolean (Variables|Default|GetEjectNow) (Variables|Default|GetFirstKey) (Variables|Default|GetSecondKey) (Variables|Default|GetThirdKey))
    (Game|OpenLevel(byName) "EndScreen")))

(event EventBeginPlay
  ;[1 1 1] Eject key input
  (Input|EnableInput (Game|GetPlayerController 0)))

(event Input|KeyboardEvents|E
  (params (Key :type Key%20Structure))
  ;[1 1 1] Eject key input
  (:Pressed
    (if (Variables|Default|GetEjectNow)
      (Variables|Default|SetFirstKey true))))

(event Input|KeyboardEvents|J
  (params (Key :type Key%20Structure))
  ;[1 1 1] Eject key input
  (:Pressed
    (if (Variables|Default|GetEjectNow)
      (Variables|Default|SetSecondKey true))))

(event Input|KeyboardEvents|C
  (params (Key :type Key%20Structure))
  ;[1 1 1] Eject key input
  (:Pressed
    (if (Variables|Default|GetEjectNow)
      (Variables|Default|SetThirdKey true))))

(fn ConstructionScript)